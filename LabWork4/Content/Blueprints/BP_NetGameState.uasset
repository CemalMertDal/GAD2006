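; Networked game state Blueprint that handles the end of a team match and its restart.
; On victory it finds the winning player's team and tells each player's avatar whether it won or lost.
; It then shows a results widget naming the winning team, adding the closest miss distance to Blue for a local Red player who is not the winner.
; Restart removes that widget.
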(event `self.OnVictory`
  (bind _returnvalue (`self.GetPlayerStateByIndex` (`self.WinningPlayer`)))
  (for _array_element (`self.PlayerArray`)
    (bind _asnet_player_state (cast `NetPlayerState` _array_element))
    (bind (_data_nickname _data_customizationdata _data_teamid) (break `SPlayerInfo` (`NetPlayerState.Data` _asnet_player_state)))
    (if (`|EnumEquality` _data_teamid (`.TeamID` (break `SPlayerInfo` (`NetPlayerState.Data` _returnvalue))))
      (bind _asbp_net_avatar (cast `/Game/Blueprints/BP_NetAvatar` (`PlayerState.PawnPrivate` _asnet_player_state) :!pure true))
      (`/Game/Blueprints/BP_NetAvatar.OnPlayerWon` _asbp_net_avatar)
      (else
        (`/Game/Blueprints/BP_NetAvatar.OnPlayerLost` _asbp_net_avatar))))
  (`self.ShowResultMessage`))

(event `self.OnRestart`
  (`Widget.RemoveFromParent` (`self.MessageWidget`)))

(fn `ShowResultMessage`
  (bind _playerstate (`Controller.PlayerState` (`GameplayStatics.GetPlayerController` 0)))
  (bind _asnet_player_state (cast `NetPlayerState` _playerstate :!pure true))
  (bind (_data_nickname _data_customizationdata _data_teamid) (break `SPlayerInfo` (`NetPlayerState.Data` _asnet_player_state)))
  (bind _returnvalue (`self.GetPlayerStateByIndex` (`self.WinningPlayer`)))
  (bind _returnvalue_2 (`|CreateWidget` "/Game/Blueprints/UMG/W_GameResults.W_GameResults_C" null (`|FormatText` "{team} WINS!" (`|GetEnumeratorNameAsString` (`.TeamID` (break `SPlayerInfo` (`NetPlayerState.Data` _returnvalue))))) (select `bool` (and (not (== _returnvalue _playerstate)) (`|EnumEquality` _data_teamid "TEAM_Red")) :`true` (`|FormatText` "Missed by {distance}m!" (`KismetTextLibrary.Conv_DoubleToText` (/ (`NetPlayerState.ClosestApproachToBlue` _asnet_player_state) 100.0) "HalfToEven" false true 1 324 0 1)))))
  (bind _output_get (set `self.MessageWidget` _returnvalue_2))
  (`UserWidget.AddToViewport` _output_get 0))

(fn `UserConstructionScript`)